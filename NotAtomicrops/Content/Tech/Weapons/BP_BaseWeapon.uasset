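; Base weapon actor that fires projectiles through weapon interface events, limited by the owner's inventory ammo.
; Init caches the owner and its inventory; firing checks ammo, plays sound, spawns the effect and a scaled-down projectile ahead of an Arrow component, then decrements ammo.
; The projectile's owner is the instigator's controller.
; The empty-fire function is a stub, and an interface getter exposes the weapon delay.
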(event `/Game/Tech/Weapons/I_WeaponInterface.I_WeaponInit`
  (params (Owner :type "Actor Object Reference"))
  (bind _output_get (set `self.OwningActor` Owner))
  (bind _inventory (message `/Game/Tech/Interfaces/I_Player.GetInventory` _output_get))
  (set `self.PlayerInventory` _inventory))

(event `/Game/Tech/Weapons/I_WeaponInterface.I_WeaponFired`
  (params (Instigator :type "Pawn Object Reference") (Scale :type "Vector Structure") (Location :type "Vector Structure"))
  (bind (_location _rotation) (`self.SpawnProjectile`))
  ;[1 1 1] Added by a designer (gross)
  (bind _hasammo (`/Game/Tech/ActorComponents/AC_Inventory.CheckAmmo` (`self.PlayerInventory`)))
  (if _hasammo
    (`self.PlayFiring`)
    (set `self.WeaponInstigator` Instigator)
    (`GameplayStatics.SpawnEmitterAtLocation` (`self.FireEffect`) Location (`self.K2_GetActorRotation` (`self.WeaponInstigator`)) Scale)
    (`|SpawnActorFromClass` (`self.Projectile`) (`KismetMathLibrary.MakeTransform` _location _rotation (0.1 0.1 0.1)) "Undefined" "OverrideRootScale" (`Pawn.GetController` (`self.WeaponInstigator`)) 3.0 (`self.WeaponInstigator`))
    (`/Game/Tech/ActorComponents/AC_Inventory.DecreaseAmmo` (`self.PlayerInventory`))
    (else
      (`self.PlayEmpty`))))

(fn `I_WeaponDelay`
  (returns (Delay :type "Float (double-precision)"))
  (return (`self.WeaponDelay`)))

(fn `PlayEmpty`)

(fn `PlayFiring`
  (`GameplayStatics.PlaySoundAtLocation` (`self.WeaponFireSound`) (`self.K2_GetActorLocation`) (struct) 1.0 1.0 0.0 null null null))

(fn `SpawnProjectile`
  (returns (Location :type "Vector Structure") (Rotation :type "Rotator Structure"))
  (bind _arrow (`self.Arrow`))
  (return (+ (`SceneComponent.K2_GetComponentLocation` _arrow) (* (`SceneComponent.GetForwardVector` _arrow) 100.0)) (`SceneComponent.K2_GetComponentRotation` _arrow)))

(fn `UserConstructionScript`)