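; BP_Pistol is a pistol weapon that fires projectiles when it receives the IWeaponFired event.
; It checks ammo through PlayerInventory, then plays firing feedback, spawns a scaled fire effect at the Arrow and decrements ammo.
; The half-scale projectile takes its transform from SpawnProjectile, with the shooter as Instigator and the shooter's controller as Owner.
; With no ammo, it calls PlayEmpty instead.
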(event `/Game/Tech/Weapons/I_WeaponInterface.I_WeaponFired`
  (params (Instigator :type "Pawn Object Reference") (Scale :type "Vector Structure") (Location :type "Vector Structure"))
  (bind (_location _rotation) (`self.SpawnProjectile`))
  (bind _hasammo (`/Game/Tech/ActorComponents/AC_Inventory.CheckAmmo` (`self.PlayerInventory`)))
  (if _hasammo
    (`self.PlayFiring`)
    (set `self.WeaponInstigator` Instigator)
    (`GameplayStatics.SpawnEmitterAtLocation` (`self.FireEffect`) (`SceneComponent.K2_GetComponentLocation` (`self.Arrow`)) (`self.K2_GetActorRotation` (`self.WeaponInstigator`)) Scale)
    (`|SpawnActorFromClass` (`self.Projectile`) (`KismetMathLibrary.MakeTransform` _location _rotation (0.5 0.5 0.5)) "Undefined" "OverrideRootScale" (`Pawn.GetController` (`self.WeaponInstigator`)) 3.0 0.0 (`self.WeaponInstigator`))
    (`/Game/Tech/ActorComponents/AC_Inventory.DecreaseAmmo` (`self.PlayerInventory`))
    (else
      (`self.PlayEmpty`))))

(fn `UserConstructionScript`
  (`parent.UserConstructionScript`))