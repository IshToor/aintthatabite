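; BP_RepairTool is a hold-to-fire tool that repeatedly launches a projectile while the trigger is held.
; The hold-fire interface event opens and enters a Gate, which plays a fire effect and spawns a scaled-down projectile owned by the instigator's controller.
; A Delay re-enters the Gate to loop at the weapon's fire interval until the release event closes it.
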(event `/Game/Tech/Weapons/I_WeaponInterface.I_HoldWeaponFired`
  (params (Instigator :type "Pawn Object Reference") (Scale :type "Vector Structure") (Location :type "Vector Structure"))
  (bind (_location _rotation) (`self.SpawnProjectile`))
  (`|ExecutionSequence`
    (:`then_0`
      (goto _label :!via `Open`))
    (:`then_1`
      (`/Engine/EditorBlueprintResources/StandardMacros.Gate` true :!label _label
        (:`Exit`
          (set `self.WeaponInstigator` Instigator)
          (`GameplayStatics.SpawnEmitterAtLocation` (`self.FireEffect`) Location (`self.K2_GetActorRotation` (`self.WeaponInstigator`)) Scale)
          (`|SpawnActorFromClass` (`self.Projectile`) (`KismetMathLibrary.MakeTransform` _location _rotation (0.1 0.1 0.1)) "Undefined" "OverrideRootScale" (`Pawn.GetController` (`self.WeaponInstigator`)) (`self.WeaponInstigator`))
          (`KismetSystemLibrary.Delay` (`self.WeaponDelay`))
          (goto _label))))))

(event `/Game/Tech/Weapons/I_WeaponInterface.I_ReleaseWeaponFire`
  (goto _label :!via `Close`))

(fn `UserConstructionScript`
  (`parent.UserConstructionScript`))