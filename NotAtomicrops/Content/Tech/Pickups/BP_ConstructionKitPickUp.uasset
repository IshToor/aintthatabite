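; BP_ConstructionKitPickUp is a pickup that grants construction kits to the player who activates it.
; Activate stores the player and, if it implements I_Pickup, sends the increase amount through the OnConstructionKitPickUpMessage interface call.
; It returns whether the interface was found and prints a debug string either way.
; The event graph holds only disabled default events, so all logic lives in Activate.
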(fn `Activate`
  (params (Player :type "Actor Object Reference"))
  (returns (Success :type Boolean))
  (locals (PlayerRef :type "Actor Object Reference"))
  (bind _output_get (set `local.PlayerRef` Player))
  (bind _returnvalue (`KismetSystemLibrary.DoesImplementInterface` _output_get "/Game/Tech/Interfaces/I_Pickup.I_Pickup_C"))
  (if _returnvalue
    (message `/Game/Tech/Interfaces/I_Pickup.OnConstructionKitPickUp` (`local.PlayerRef`) (`self.ConstructionKitIncreaseAmount`))
    (`KismetSystemLibrary.PrintString` "Player has interface" true true (struct :`R` 0.110038 :`G` 1.0 :`A` 1.0) 10.0)
    (else
      (`KismetSystemLibrary.PrintString` "Player doesn't have interface" true true (struct :`R` 1.0 :`G` 0.028078 :`A` 1.0) 10.0)))
  (return _returnvalue))

(fn `UserConstructionScript`
  (`parent.UserConstructionScript`))