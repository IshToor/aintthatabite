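; Projectile fired by the repair tool, which applies its Damage value to turrets and a small fixed damage to anything else it hits.
; A DoOnce on the Hit event limits it to one impact, crediting OwningController as instigator before the projectile destroys itself.
; The turret check is an exact class comparison, so subclasses of Turret receive the small fixed amount.
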(event `self.ReceiveHit`
  (params (MyComp :type "PrimitiveComponent Object Reference") (Other :type "Actor Object Reference") (OtherComp :type "PrimitiveComponent Object Reference") (bSelfMoved :type Boolean) (HitLocation :type "Vector Structure") (HitNormal :type "Vector Structure") (NormalImpulse :type "Vector Structure") (Hit :type "HitResult Structure (by ref)"))
  (`/Engine/EditorBlueprintResources/StandardMacros.DoOnce` false
    (:`Completed`
      (bind _output_get (set `self.DamagedActor` Other))
      (if (!= _output_get null)
        (if (!= (`GameplayStatics.GetObjectClass` (`self.DamagedActor`)) "/Game/Tech/Defenses/Turret.Turret_C")
          (`GameplayStatics.ApplyDamage` (`self.DamagedActor`) 0.25 (`self.owningController`) self)
          (`self.K2_DestroyActor`)
          (else
            (`GameplayStatics.ApplyDamage` (`self.DamagedActor`) (`self.damage`) (`self.owningController`) self)
            (`self.K2_DestroyActor`)))
        (else
          (`self.K2_DestroyActor`))))))

(fn `UserConstructionScript`
  (`parent.UserConstructionScript`))