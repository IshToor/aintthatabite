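; BP_AOEProjectile_Child is a child projectile Blueprint that deals area-of-effect damage on impact.
; Its first Hit event, gated by DoOnce, checks the hit actor, applies radial damage with falloff around the projectile if that passes, then destroys itself either way.
; Damage, falloff and instigating controller come from variables, while the owner and first player controller are passed as ignored actors.
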(event `self.ReceiveHit`
  (params (MyComp :type "PrimitiveComponent Object Reference") (Other :type "Actor Object Reference") (OtherComp :type "PrimitiveComponent Object Reference") (bSelfMoved :type Boolean) (HitLocation :type "Vector Structure") (HitNormal :type "Vector Structure") (NormalImpulse :type "Vector Structure") (Hit :type "HitResult Structure (by ref)"))
  (`/Engine/EditorBlueprintResources/StandardMacros.DoOnce` false
    (:`Completed`
      (bind _output_get (set `self.DamagedActor` Other))
      (if (!= _output_get null)
        (`GameplayStatics.ApplyRadialDamageWithFalloff` (`self.damage`) 1.0 (`self.K2_GetActorLocation`) 50.0 200.0 (`self.DamageDropOff`) null (`|MakeArray` (`GameplayStatics.GetPlayerController` 0) (`self.GetOwner` self) :!type "Actor Object Reference") self (`self.owningController`))
        (`self.K2_DestroyActor`)
        (else
          (`self.K2_DestroyActor`))))))

(fn `UserConstructionScript`
  (`parent.UserConstructionScript`))