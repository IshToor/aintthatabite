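; Base projectile actor that deals damage to whatever it hits and then destroys itself.
; On its first Hit event, guarded by DoOnce, it applies damage to a non-null hit actor, crediting the owning controller as instigator.
; Damage comes from the owner's TurretDamage when the owner is a Turret, otherwise from the projectile's own Damage value.
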(event `self.ReceiveHit`
  (params (MyComp :type "PrimitiveComponent Object Reference") (Other :type "Actor Object Reference") (OtherComp :type "PrimitiveComponent Object Reference") (bSelfMoved :type Boolean) (HitLocation :type "Vector Structure") (HitNormal :type "Vector Structure") (NormalImpulse :type "Vector Structure") (Hit :type "HitResult Structure (by ref)"))
  (bind _owningcontroller (`self.owningController`))
  (bind _damagedactor (`self.DamagedActor`))
  (`/Engine/EditorBlueprintResources/StandardMacros.DoOnce` false
    (:`Completed`
      (bind _output_get (set `self.DamagedActor` Other))
      (if (!= _output_get null)
        (bind _asturret (cast `/Game/Tech/Defenses/Turret` (`self.GetOwner` self))
          (:`then`
            (`GameplayStatics.ApplyDamage` _damagedactor (`/Game/Tech/Defenses/Turret.TurretDamage` _asturret) _owningcontroller self))
          (:`CastFailed`
            (`GameplayStatics.ApplyDamage` _damagedactor (`self.damage`) _owningcontroller self)))
        (`self.K2_DestroyActor`)
        (else
          (`self.K2_DestroyActor`))))))

(fn `UserConstructionScript`)