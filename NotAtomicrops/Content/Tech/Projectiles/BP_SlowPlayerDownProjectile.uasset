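; BP_SlowPlayerDownProjectile is a projectile that slows the player it hits.
; Its Hit event runs through a DoOnce, so only the first hit counts.
; A BP_NewTopDownShooter hit gets SlowPlayerDownEvent called on it, then the projectile destroys itself.
; A hit without an actor also destroys it, while any other actor fails the cast and leaves the projectile alive but spent.
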(event `self.ReceiveHit`
  (params (MyComp :type "PrimitiveComponent Object Reference") (Other :type "Actor Object Reference") (OtherComp :type "PrimitiveComponent Object Reference") (bSelfMoved :type Boolean) (HitLocation :type "Vector Structure") (HitNormal :type "Vector Structure") (NormalImpulse :type "Vector Structure") (Hit :type "HitResult Structure (by ref)"))
  (`/Engine/EditorBlueprintResources/StandardMacros.DoOnce` false
    (:`Completed`
      (bind _output_get (set `self.DamagedActor` Other))
      (if (!= _output_get null)
        (bind _asbp_new_top_down_shooter (cast `/Game/Tech/PlayerCharacter/BP_NewTopDownShooter` (`self.DamagedActor`)))
        (`/Game/Tech/PlayerCharacter/BP_NewTopDownShooter.SlowPlayerDownEvent` _asbp_new_top_down_shooter)
        (`self.K2_DestroyActor`)
        (else
          (`self.K2_DestroyActor`))))))

(fn `UserConstructionScript`
  (`parent.UserConstructionScript`))