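; Tutorial shambler enemy that wanders endlessly between a set of walking points.
; On BeginPlay it shuffles the WalkingPoints array and uses AI MoveTo to walk to the first entry's location.
; Each successful arrival reshuffles and moves again, so the same point can repeat, and a failed move ends the loop.
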(event `ShuffleLocations`
  (`KismetArrayLibrary.Array_Shuffle` (`self.WalkingPoints`))
  (`self.MoveTo`))

(event `self.ReceiveBeginPlay`
  (`self.ShuffleLocations`))

(event `MoveTo`
  (`|AIMoveTo` self (`SceneComponent.K2_GetComponentLocation` (`/Game/Tech/AI/TutorialAI/WalkingPoint.DefaultSceneRoot` (`|GetArrayItem` (`self.WalkingPoints`)))) null
    (:`OnSuccess`
      (`self.ShuffleLocations`))))

(fn `UserConstructionScript`
  (`parent.UserConstructionScript`))