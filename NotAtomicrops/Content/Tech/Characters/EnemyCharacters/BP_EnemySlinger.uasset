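; BP_EnemySlinger is an enemy character that performs an animated ranged attack.
; FireWeapon plays the slinger fire sound at the actor's location and starts the attack montage on its mesh.
; The montage's Attack notify sends IWeaponFiredMessage to the child actor, timing the shot to the animation.
; SetupAIAgent sets the navigation agent's radius and height, and construction defers to the parent class.
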(event `FireWeapon`
  (`GameplayStatics.PlaySoundAtLocation` "/Game/Audio/Slingerfire.Slingerfire" (`self.K2_GetActorLocation`) (struct) 1.0 1.0 0.0 null null null)
  (bind _notifyname (`|PlayMontage` (`self.Mesh`) (`self.AttackAnim`))
    (:`OnNotifyBegin`
      (switch `name` _notifyname
        (:`Attack`
          (message `/Game/Tech/Weapons/I_WeaponInterface.I_WeaponFired` (`ChildActorComponent.ChildActor` (`self.ChildActor`)) null (1.0 1.0 1.0) (0.0 0.0 0.0)))))))

(fn `SetupAIAgent`
  (set `NavMovementComponent.NavAgentProps` (make `NavAgentProperties` 35.0 144.0) (`self.CharacterMovement`)))

(fn `UserConstructionScript`
  (`parent.UserConstructionScript`))