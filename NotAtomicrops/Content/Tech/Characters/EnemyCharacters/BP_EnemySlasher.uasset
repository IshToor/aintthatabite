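; BP_EnemySlasher is a melee enemy character that slashes a turret passed to its Attack event.
; Attack is gated by CanAttack, then plays a slash sound and the attack montage.
; The montage's Attack notify applies damage to the turret, timing the hit to the animation.
; When the montage completes, a delay of AttackRate re-enables attacking; BeginPlay and construction defer to the parent class.
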(event `self.ReceiveBeginPlay`
  (`parent.ReceiveBeginPlay`))

(event `Attack`
  (params (Turret :type "Actor Object Reference"))
  (if (`self.CanAttack`)
    (set `self.CanAttack` false)
    (`GameplayStatics.PlaySoundAtLocation` "/Game/Audio/ZombieSlash.ZombieSlash" (`self.K2_GetActorLocation`) (struct) 1.0 1.0 0.0 null null null)
    (bind _notifyname (`|PlayMontage` (`self.Mesh`) (`self.AttackAnim`))
      (:`OnCompleted`
        (`KismetSystemLibrary.Delay` (`self.AttackRate`))
        (set `self.CanAttack` true))
      (:`OnNotifyBegin`
        (switch `name` _notifyname
          (:`Attack`
            (`GameplayStatics.ApplyDamage` Turret (`self.Damage`) null self)))))))

(fn `UserConstructionScript`
  (`parent.UserConstructionScript`))