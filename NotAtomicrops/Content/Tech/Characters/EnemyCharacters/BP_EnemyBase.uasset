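; Base enemy character, apparently a zombie, that attacks nearby actors and reports its death to the wave manager and game mode for points.
; Damage and healing route through the ACHealth component.
; Freeze slows movement and Burn applies delay-throttled damage from Tick, each with particle effects and timed decay.
; Sphere overlap starts a looping attack timer, cleared on exit; BaseAttack applies damage on a montage notify, gated by an attack-rate cooldown.
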(event `self.ReceiveBeginPlay`
  (`GameplayStatics.SpawnSoundAttached` "/Game/Audio/ZombieBreathing.ZombieBreathing" (`self.CapsuleComponent`) "None" (0.0 0.0 0.0) (struct) "KeepRelativeOffset" true 0.3 1.0 0.0 null null))

(event `self.ReceiveAnyDamage`
  (params (Damage :type "Float (single-precision)") (DamageType :type "DamageType Object Reference") (InstigatedBy :type "Controller Object Reference") (DamageCauser :type "Actor Object Reference"))
  (bind _niagara (`self.Niagara`))
  ;[0 1 0.1332] Added by Josh
  (`NiagaraComponent.ResetSystem` _niagara)
  (`ActorComponent.Activate` _niagara false)
  (bind _dead (`/Game/Tech/ActorComponents/AC_Health.TakeDamage` (`self.AC_Health`) Damage))
  (if _dead
    (`self.OnDeath`)))

(event `OnDeath`
  (`/Game/Tech/Managers/WavesManager.OnAIDeath` (`/Game/Tech/GameModes/WaveBasedGameMode.WavesManagerRef` (`/Game/Tech/Controllers/MyAIController.GameMode` (`self.AIController`))) self)
  (`/Game/Tech/GameModes/WaveBasedGameMode.Targetpoints` (`/Game/Tech/Controllers/MyAIController.GameMode` (`self.AIController`)) (`self.Points`))
  (`self.K2_DestroyActor`))

(event `OnHeal`
  (params (HealthRecieved :type "Float (double-precision)"))
  (`/Game/Tech/ActorComponents/AC_Health.RecieveHealth` (`self.AC_Health`) HealthRecieved)
  (`KismetSystemLibrary.PrintString` "We have received health"))

(event `/Game/Tech/Defenses/Status/StatusEffects.BeginStatusDecay`
  (params (DecayTime :type "Float (single-precision)") (StatusType :type "/Game/Tech/Defenses/Status/StatusList Enum" :default "NewEnumerator0"))
  ;[1 1 1] Status Effects
  (`KismetSystemLibrary.Delay` DecayTime)
  (switch `/Game/Tech/Defenses/Status/StatusList` StatusType
    (:`NewEnumerator0`
      (set `CharacterMovementComponent.MaxWalkSpeed` (`self.MoveSpeed`) (`self.CharacterMovement`))
      (`ActorComponent.Deactivate` (`self.FreezeSystem`)))
    (:`NewEnumerator1`
      (set `self.Burning` false)
      (`ActorComponent.Deactivate` (`self.BurningSystem`)))))

(event `/Game/Tech/Defenses/Status/StatusEffects.GetSpeedNerf`
  (params (SpeedNerf :type "Float (single-precision)"))
  ;[1 1 1] Status Effects
  (set `CharacterMovementComponent.MaxWalkSpeed` (* (`self.MoveSpeed`) SpeedNerf) (`self.CharacterMovement`))
  (`ActorComponent.Activate` (`self.FreezeSystem`) false))

(event `Init`
  ;[1 1 1] Status Effects
  (set `CharacterMovementComponent.MaxWalkSpeed` (`self.MoveSpeed`) (`self.CharacterMovement`)))

(event `/Game/Tech/Defenses/Status/StatusEffects.GetDOT`
  (params (DamageOverTime :type "Float (single-precision)") (Instigator :type "Actor Object Reference"))
  ;[1 1 1] Status Effects
  (set `self.BurnDMG` DamageOverTime)
  (if (not (`self.Burning`))
    (set `self.Burning` true)))

(event `self.ReceiveTick`
  (params (DeltaSeconds :type "Float (single-precision)"))
  ;[1 1 1] Status Effects
  (`KismetSystemLibrary.Delay` 1.0)
  (if (`self.Burning`)
    (bind _returnvalue (`GameplayStatics.ApplyDamage` self (stale `/Game/Tech/Defenses/Status/StatusEffects.GetDOT` DamageOverTime) null (stale `/Game/Tech/Defenses/Status/StatusEffects.GetDOT` Instigator)))
    (`KismetSystemLibrary.PrintString` (`KismetStringLibrary.Conv_DoubleToString` _returnvalue))
    (`ActorComponent.Activate` (`self.BurningSystem`) false)))

(event `self.Sphere.OnComponentBeginOverlap`
  (params (OverlappedComponent :type "PrimitiveComponent Object Reference") (OtherActor :type "Actor Object Reference") (OtherComp :type "PrimitiveComponent Object Reference") (OtherBodyIndex :type Integer) (bFromSweep :type Boolean) (SweepResult :type "HitResult Structure (by ref)"))
  (bind _output_get (set `self.AttackedActor` OtherActor))
  (`KismetSystemLibrary.PrintString` (`KismetStringLibrary.Concat_StrStr` "This is the attack actor: " (`KismetSystemLibrary.GetDisplayName` _output_get)))
  (`/Engine/EditorBlueprintResources/StandardMacros.DoOnce` false :!label _label
    (:`Completed`
      (bind _returnvalue (`KismetSystemLibrary.K2_SetTimerDelegate` (`|CreateDelegate` :!event `BaseAttack`) 1.0 true))
      (set `self.AttackTimer` _returnvalue))))

(event `ResetDoOnce`
  (goto _label :!via `Reset`))

(event `BaseAttack`
  (if (`self.CanAttack`)
    (set `self.CanAttack` false)
    (bind _notifyname (`|PlayMontage` (`self.Mesh`) (`self.AttackAnim`))
      (:`OnCompleted`
        (`KismetSystemLibrary.Delay` (`self.AttackRate`))
        (set `self.CanAttack` true))
      (:`OnNotifyBegin`
        (switch `name` _notifyname
          (:`Attack`
            (`GameplayStatics.ApplyDamage` (`self.AttackedActor`) (`self.Damage`) null self)))))))

(event `self.Sphere.OnComponentEndOverlap`
  (params (OverlappedComponent :type "PrimitiveComponent Object Reference") (OtherActor :type "Actor Object Reference") (OtherComp :type "PrimitiveComponent Object Reference") (OtherBodyIndex :type Integer))
  (`KismetSystemLibrary.PrintString` "Exited")
  (`KismetSystemLibrary.K2_ClearAndInvalidateTimerHandle` (`self.AttackTimer`))
  (`self.ResetDoOnce`))

(fn `UserConstructionScript`)