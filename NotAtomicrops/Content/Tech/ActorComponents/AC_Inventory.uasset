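; AC_Inventory is an actor component that tracks a weapon inventory and cycles the equipped weapon.
; EquipWeapon picks a class from the Inventory map's keys by index and passes it to the owner through ChangeWeaponMessage.
; CycleUp and CycleDown step the equipped index, wrapping at either end, then equip that weapon.
; UpdateAmmo is an empty stub, and UpdateWeaponEquipped does nothing because its logic is unconnected.
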(event `EquipWeapon`
  (params (ItemToEquip :type Integer))
  (bind _keys (`BlueprintMapLibrary.Map_Keys` (`self.Inventory`)))
  (bind _output_get (set `self.EquippedWeaponClass` (`|GetArrayItem` _keys ItemToEquip)))
  (message `/Game/Tech/Interfaces/I_Player.ChangeWeapon` (`self.GetOwner`) _output_get))

(event `CycleUp`
  (bind _result (`/Engine/EditorBlueprintResources/StandardMacros.IncrementInt` (`self.EquippedWeaponIndex`))
    (:`  `
      (bind _keys (`BlueprintMapLibrary.Map_Keys` (`self.Inventory`)))
      (if (`KismetArrayLibrary.Array_IsValidIndex` _keys _result)
        (`self.EquipWeapon` (`self.EquippedWeaponIndex`))
        (`self.UpdateWeaponEquipped`)
        (else
          (bind _output_get (set `self.EquippedWeaponIndex` 0))
          (`self.EquipWeapon` _output_get)
          (`self.UpdateWeaponEquipped`))))))

(event `CycleDown`
  (bind _result (`/Engine/EditorBlueprintResources/StandardMacros.DecrementInt` (`self.EquippedWeaponIndex`))
    (:`  `
      (bind _keys (`BlueprintMapLibrary.Map_Keys` (`self.Inventory`)))
      (if (`KismetArrayLibrary.Array_IsValidIndex` _keys _result)
        (`self.EquipWeapon` (`self.EquippedWeaponIndex`))
        (`self.UpdateWeaponEquipped`)
        (else
          (bind _output_get (set `self.EquippedWeaponIndex` (`KismetArrayLibrary.Array_LastIndex` _keys)))
          (`self.EquipWeapon` _output_get)
          (`self.UpdateWeaponEquipped`))))))

(event `UpdateAmmo`)