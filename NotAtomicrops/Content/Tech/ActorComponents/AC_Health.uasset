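; AC_Health is an actor component that tracks a health value for its owning actor.
; CurrentHealth starts at MaxHealth on BeginPlay, and TakeDamage and RecieveHealth subtract from or add to it.
; Both functions pass the result through CheckHealthWithinLimits, which clamps it between MinHealth and MaxHealth.
; TakeDamage returns true when health drops to zero or below, signalling depletion to the caller.
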(event `self.ReceiveBeginPlay`
  (set `self.CurrentHealth` (`self.MaxHealth`)))

(fn `CheckHealthWithinLimits`
  (params (Health :type "Float (double-precision)"))
  (returns (ReturnHealth :type "Float (double-precision)"))
  (return (`KismetMathLibrary.FClamp` Health (`self.MinHealth`) (`self.MaxHealth`))))

(fn `RecieveHealth`
  (params (HealthRecieved :type "Float (double-precision)"))
  (bind _returnhealth (`self.CheckHealthWithinLimits` (+ HealthRecieved (`self.CurrentHealth`))))
  (set `self.CurrentHealth` _returnhealth)
  (return))

(fn `TakeDamage`
  (params (DamageTaken :type "Float (double-precision)"))
  (returns (Dead :type Boolean))
  (bind _returnhealth (`self.CheckHealthWithinLimits` (- (`self.CurrentHealth`) DamageTaken)))
  (set `self.CurrentHealth` _returnhealth)
  (if (> _returnhealth 0.0)
    (return false)
    (else
      (return true))))