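; Purchasable defense placeholder that is replaced by a wall, decoy or bomb actor when used.
; Construction sets the mesh, sizes the trigger box to its bounds, centers it and derives the display name from the DefenseType class name.
; BeginPlay applies the purchase material and creates the prompt widget inside that per-material loop; box overlap toggles the prompt.
; Use or Option1 plays a build effect, spawns the defense, and destroys the placeholder.
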(event `self.ReceiveBeginPlay`
  (set `self.DefenseLocation` (`self.K2_GetActorLocation`))
  (bind _output_get (set `self.PurchasedMaterials` (`MeshComponent.GetMaterials` (`self.StaticMesh`))))
  (for (_ _array_index) _output_get
    (`self.ChangeMaterial` _array_index (`self.PurchaseMaterial`))
    (bind _returnvalue (`|CreateWidget` "/Game/Tech/UI/PlayerUI/PurchaseDefenceWidget.PurchaseDefenceWidget_C" (`GameplayStatics.GetPlayerController` 0)))
    (bind _output_get_2 (set `self.PurchaseDefenceUIRef` _returnvalue))
    (`/Game/Tech/UI/PlayerUI/PurchaseDefenceWidget.Init` _output_get_2)
    (`/Game/Tech/UI/PlayerUI/PurchaseDefenceWidget.UpdatePurchaseMessage` _output_get_2 (`self.DefenseTypeName`))))

(event `/Game/Tech/Interfaces/I_Interactable.Use`
  (`self.PurchasedDefense` :!label _label))

(event `/Game/Tech/Interfaces/I_Interactable.Option1`
  (goto _label))

(event `PurchasedDefense`
  (`/Engine/EditorBlueprintResources/StandardMacros.DoOnce` false
    (:`Completed`
      (`GameplayStatics.SpawnEmitterAtLocation` "/Game/Jake-Particles/BuildObstacle/Effects/FX_Breakables/Wall/FX_Build.FX_Build" (`self.K2_GetActorLocation`))
      (bind _returnvalue (`|SpawnActorFromClass` (`self.DefenseType`) (`self.GetTransform`) "AlwaysSpawn" "OverrideRootScale" null (`self.Mesh`) null))
      (message `/Game/Tech/Interfaces/I_Defence.Activate` _returnvalue)
      (`self.K2_DestroyActor`))))

(event `self.Box.OnComponentBeginOverlap`
  (params (OverlappedComponent :type "PrimitiveComponent Object Reference") (OtherActor :type "Actor Object Reference") (OtherComp :type "PrimitiveComponent Object Reference") (OtherBodyIndex :type Integer) (bFromSweep :type Boolean) (SweepResult :type "HitResult Structure (by ref)"))
  (`UserWidget.AddToViewport` (`self.PurchaseDefenceUIRef`) 0))

(event `self.Box.OnComponentEndOverlap`
  (params (OverlappedComponent :type "PrimitiveComponent Object Reference") (OtherActor :type "Actor Object Reference") (OtherComp :type "PrimitiveComponent Object Reference") (OtherBodyIndex :type Integer))
  (`Widget.RemoveFromParent` (`self.PurchaseDefenceUIRef`)))

(event `OnActivate`)

(fn `ChangeMaterial`
  (params (Index :type Integer) (ChangeTo :type "MaterialInterface Object Reference"))
  (`PrimitiveComponent.SetMaterial` (`self.StaticMesh`) Index ChangeTo))

(fn `UserConstructionScript`
  (bind (_min _max) (`StaticMeshComponent.GetLocalBounds` (`self.StaticMesh`)))
  (`StaticMeshComponent.SetStaticMesh` (`self.StaticMesh`) (`self.Mesh`))
  (`BoxComponent.SetBoxExtent` (`self.Box`) (`.BoxExtent` (`KismetSystemLibrary.GetComponentBounds` (`self.StaticMesh`))) true)
  (`SceneComponent.K2_AddLocalOffset` (`self.StaticMesh`) (* (/ (+ _min _max) 2) -1) false false)
  (switch `name` (`KismetStringLibrary.Conv_StringToName` (`KismetSystemLibrary.GetClassDisplayName` (`self.DefenseType`)))
    (:`Default`
      (`KismetSystemLibrary.PrintString` "Apparently None Of These!!!!" true true (struct :`R` 1.0 :`A` 1.0) 1.0))
    (:`Wall_C`
      (set `self.DefenseTypeName` "Wall"))
    (:`Decoy_C`
      (set `self.DefenseTypeName` "Decoy"))
    (:`Bomb_C`
      (set `self.DefenseTypeName` "Bomb"))))