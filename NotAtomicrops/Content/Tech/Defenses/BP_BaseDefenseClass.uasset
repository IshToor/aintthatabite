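; Base class for defenses: damageable actors with a configurable mesh and a world-space health bar.
; The construction script applies the mesh, sizes the box to its bounds and recenters it.
; Damage passes through ACHealth and refreshes the bar, spawning an explosion and destroying the actor when TakeDamage returns true.
; Helpers swap materials and yaw the bar toward the player, and activation re-caches the explosion location.
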(event `self.ReceiveBeginPlay`
  (set `self.DefenseLocation` (`self.K2_GetActorLocation`))
  (bind _asuniversal_health_bar (cast `/Game/UniversalHealthBar` (`WidgetComponent.GetUserWidgetObject` (`self.HealthBarWidget`)))
    (:`then`
      (bind _output_get (set `self.HealthBar` _asuniversal_health_bar))
      (set `/Game/UniversalHealthBar.HealthSystem` (`self.AC_Health`) _output_get)
      (`/Game/UniversalHealthBar.Init` (`self.HealthBar`))
      (`/Game/UniversalHealthBar.UpdateHealthBar` (`self.HealthBar`)))
    (:`CastFailed`
      (`KismetSystemLibrary.PrintString` "How is this failing?!" true true (struct :`R` 1.0 :`G` 0.044042 :`A` 1.0) 10.0))))

(event `Destroyed`
  (`GameplayStatics.SpawnEmitterAtLocation` "/Game/StarterContent/Particles/P_Explosion.P_Explosion" (`self.DefenseLocation`) (struct) (3.0 3.0 3.0))
  (`self.K2_DestroyActor`))

(event `OnActivate`
  (set `self.DefenseLocation` (`self.K2_GetActorLocation`)))

(event `self.ReceiveAnyDamage`
  (params (Damage :type "Float (single-precision)") (DamageType :type "DamageType Object Reference") (InstigatedBy :type "Controller Object Reference") (DamageCauser :type "Actor Object Reference"))
  (bind _dead (`/Game/Tech/ActorComponents/AC_Health.TakeDamage` (`self.AC_Health`) Damage))
  (`/Game/UniversalHealthBar.UpdateHealthBar` (`self.HealthBar`))
  (if _dead
    (`self.Destroyed`)))

(event `/Game/Tech/Interfaces/I_Defence.Activate`
  (`self.OnActivate`))

(fn `ChangeMaterial`
  (params (Index :type Integer) (ChangeTo :type "MaterialInterface Object Reference"))
  (`PrimitiveComponent.SetMaterial` (`self.StaticMesh`) Index ChangeTo))

(fn `GetRotationToPlayer`
  (returns (ReturnValue :type "Rotator Structure"))
  (bind _returnvalue (`GameplayStatics.GetPlayerController` 0))
  (bind _returnvalue_2 (`Controller.K2_GetPawn` _returnvalue))
  (bind (_returnvalue_roll _returnvalue_pitch _returnvalue_yaw) (`KismetMathLibrary.BreakRotator` (`KismetMathLibrary.Conv_VectorToRotator` (- (`self.K2_GetActorLocation` _returnvalue_2) (`SceneComponent.K2_GetComponentLocation` (`self.HealthBarWidget`))))))
  (`/Engine/EditorBlueprintResources/StandardMacros.IsValid` _returnvalue
    (:`Is Valid`
      (`/Engine/EditorBlueprintResources/StandardMacros.IsValid` _returnvalue_2
        (:`Is Valid`
          (return (`KismetMathLibrary.MakeRotator` 0.0 0.0 _returnvalue_yaw)))
        (:`Is Not Valid`
          _)))
    (:`Is Not Valid`
      _))
  (return))

(fn `RotateHealthBarToPlayer`
  (if (!= (`SceneComponent.K2_GetComponentRotation` (`self.HealthBarWidget`)) (`self.GetRotationToPlayer`) :`ErrorTolerance` 1.0)
    (`SceneComponent.K2_SetWorldRotation` (`self.HealthBarWidget`) (`self.GetRotationToPlayer`) false false)))

(fn `UserConstructionScript`
  (bind (_min _max) (`StaticMeshComponent.GetLocalBounds` (`self.StaticMesh`)))
  (`StaticMeshComponent.SetStaticMesh` (`self.StaticMesh`) (`self.Mesh`))
  (`BoxComponent.SetBoxExtent` (`self.Box`) (`.BoxExtent` (`KismetSystemLibrary.GetComponentBounds` (`self.StaticMesh`))) true)
  (`SceneComponent.K2_AddLocalOffset` (`self.StaticMesh`) (* (/ (+ _min _max) 2) -1) false false))